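; Blood effect actor that turns exported Niagara particle data into blood decals.
; On BeginPlay it passes itself to the Niagara component's User.Data variable to receive particle callbacks.
; Each received particle spawns a BP_Decal at its position, oriented from its velocity, with randomized scale.
; The actor forwards material, fade and blot settings, and uses the particle's Size field as the decal's particle lifetime.
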(event `self.ReceiveBeginPlay`
  (`NiagaraComponent.SetNiagaraVariableObject` (`self.BloodVFXComponent`) "User.Data" self))

(event `self.ReceiveParticleData`
  (params (Data :type "Array of BasicParticleData Structure (by ref)") (NiagaraSystem :type "NiagaraSystem Object Reference"))
  (for _array_element Data
    (bind (_position _size _velocity) (break `BasicParticleData` _array_element))
    (`|SpawnActorFromClass` "/Game/Blood_VFX_Pack/Blueprints/BP_Decal.BP_Decal_C" (`KismetMathLibrary.MakeTransform` _position (`KismetMathLibrary.MakeRotFromZY` _velocity (`KismetMathLibrary.Cross_VectorVector` (`KismetMathLibrary.Normal` _velocity) (`KismetMathLibrary.Normal` (- _position (`SceneComponent.K2_GetComponentLocation` (`self.BloodVFXComponent`)))))) (* (`KismetMathLibrary.MakeVector` (`KismetMathLibrary.RandomFloatInRange` 0.9 1.3) (`KismetMathLibrary.RandomFloatInRange` 0.9 1.3) (`KismetMathLibrary.RandomFloatInRange` 0.9 1.3)) (`self.DecalScale`))) "Undefined" "OverrideRootScale" null (`self.Fade in Duration`) (`self.Start Delay`) (`self.Fade Duration`) (`self.Decal Material`) _size (`self.Blots`) null)))

(fn `UserConstructionScript`)