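; Decal actor that displays a randomized blot or line mark, fading in and out before destroying itself.
; On BeginPlay it creates a dynamic material instance with random flipbook image and distortion parameters.
; The Blots flag selects texture channel, scale and roll: blots vary randomly, while lines shrink as ParticleLifeTime rises and may flip 180 degrees.
; The construction script configures fade timing, and ParticleLifeTime also feeds the material.
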(event `self.ReceiveBeginPlay`
  (bind _decal (`self.Decal`))
  (bind _decal_2 (`self.Decal`))
  (bind _decal_3 (`self.Decal`))
  (bind _decal_4 (`self.Decal`))
  (bind _particlelifetime (`self.ParticleLifeTime`))
  (bind (_returnvalue_x _returnvalue_y _returnvalue_z) (`KismetMathLibrary.BreakVector` (`SceneComponent.K2_GetComponentScale` _decal_3)))
  ;[1 1 1] Initialization
  (`self.K2_AddActorLocalRotation` (`KismetMathLibrary.MakeRotator` 45.0))
  (`DecalComponent.SetDecalMaterial` _decal (`self.DecalMaterial`))
  (bind _returnvalue (`DecalComponent.CreateDynamicMaterialInstance` _decal))
  (bind _output_get (set `self.DynamicMat` _returnvalue))
  ;[1 1 1] Flipbook : Random Texture
  (`MaterialInstanceDynamic.SetScalarParameterValue` _output_get "Image" (`KismetMathLibrary.RandomFloatInRange` 0.0 1.0))
  (`|ExecutionSequence`
    (:`then_0`
      ;[1 1 1] Random Parameters
      (`MaterialInstanceDynamic.SetScalarParameterValue` _output_get "DistortionPower" (`KismetMathLibrary.RandomFloatInRange` 0.0 0.1))
      (`MaterialInstanceDynamic.SetScalarParameterValue` _output_get "DistortionTiling" (`KismetMathLibrary.RandomFloatInRange` 2.0 3.0))
      (`MaterialInstanceDynamic.SetScalarParameterValue` _output_get "DistortionOffset" (`KismetMathLibrary.RandomFloatInRange` 0.0 1.0)))
    (:`then_1`
      (if (`self.Blots`)
        ;[1 1 1] Blots
        (`MaterialInstanceDynamic.SetScalarParameterValue` _output_get "TextureChannel" 1.0)
        (`MaterialInstanceDynamic.SetScalarParameterValue` _output_get "TextureLifetime" (`self.ParticleLifeTime`))
        (`SceneComponent.SetWorldScale3D` _decal_3 (`KismetMathLibrary.MakeVector` _returnvalue_x _returnvalue_y (* _returnvalue_z (`KismetMathLibrary.RandomFloatInRange` 0.8 1.2))))
        (`SceneComponent.SetWorldScale3D` _decal_4 (* (`SceneComponent.K2_GetComponentScale` _decal_4) (`KismetMathLibrary.RandomFloatInRange` 0.7 1.0)))
        (`self.K2_AddActorLocalRotation` (`KismetMathLibrary.MakeRotator` (`KismetMathLibrary.RandomFloatInRange` 0.0 360.0)))
        (else
          ;[1 1 1] Line
          (`MaterialInstanceDynamic.SetScalarParameterValue` _output_get "TextureChannel" 2.0)
          (`MaterialInstanceDynamic.SetScalarParameterValue` _output_get "TextureLifetime" _particlelifetime)
          (`SceneComponent.SetWorldScale3D` _decal_2 (* (`SceneComponent.K2_GetComponentScale` _decal_2) (+ (- 1.0 _particlelifetime) 0.3)))
          (if (`KismetMathLibrary.RandomBool`)
            (`self.K2_AddActorLocalRotation` (`KismetMathLibrary.MakeRotator` 180.0))))))))

(fn `UserConstructionScript`
  (bind _decal (`self.Decal`))
  (`DecalComponent.SetFadeIn` _decal 0.0 (`self.FadeInDuration`))
  (`DecalComponent.SetFadeOut` _decal (`self.Start Delay`) (`self.FadeDuration`) true))